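; Player state that tracks energy, collected pickups and killed enemies, and owns the main HUD showing them.
; On BeginPlay it creates the HUD, restores both counters from the GameInstance if saved data exists, and refills energy to maximum.
; Gameplay events update values and HUD, firing dispatchers for door opening and death at zero energy.
; The GameInstance's save dispatcher triggers writing the counters back; energy is not persisted.
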(event `self.ReceiveBeginPlay`
  (bind _returnvalue (`|CreateWidget` "/Game/Customs/Blueprints/UI/Widget/WBP_MainHud.WBP_MainHud_C"))
  (bind _output_get (set `self.HudRef` _returnvalue))
  (`UserWidget.AddToViewport` _output_get 0)
  (bind _asbp_game_instance (cast `/Game/Customs/Blueprints/GameplayFrameWork/BP_GameInstance` (`GameplayStatics.GetGameInstance`)))
  (bind _output_get_2 (set `self.GameInstanceRef` _asbp_game_instance))
  (add `/Game/Customs/Blueprints/GameplayFrameWork/BP_GameInstance.DispatcherSave` _output_get_2 (delegate `DispatcherSave`))
  (if (not (`BlueprintMapLibrary.Map_IsEmpty` (`/Game/Customs/Blueprints/GameplayFrameWork/BP_GameInstance.PlayerStateData` _output_get_2)))
    (`self.Load`))
  (set `self.Energy` (`self.MaxEnergy`))
  (`self.UpdateHealthBar`)
  (`self.UpdateHudArchivement`))

(event `DispatcherSave`
  (`self.Save`))

(event `PickUpCollectible`
  (set `self.CollectiblesNumber` (+ (`self.CollectiblesNumber`) 1))
  (`self.UpdateHudArchivement`)
  (`self.DispatcherOpen`))

(event `KillEnemy`
  (set `self.EnemiesNumber` (+ (`self.EnemiesNumber`) 1))
  (`self.UpdateHudArchivement`)
  (`self.DispatcherOpen`))

(event `Save`
  (`BlueprintMapLibrary.Map_Add` (`/Game/Customs/Blueprints/GameplayFrameWork/BP_GameInstance.PlayerStateData` (`self.GameInstanceRef`)) 0 (make `/Game/Customs/Blueprints/GameplayFrameWork/DataStructs/BPS_PlayerStateData` (`self.CollectiblesNumber`) (`self.EnemiesNumber`))))

(event `Load`
  (bind (_value _returnvalue) (`BlueprintMapLibrary.Map_Find` (`/Game/Customs/Blueprints/GameplayFrameWork/BP_GameInstance.PlayerStateData` (`self.GameInstanceRef`))))
  (if _returnvalue
    (set `self.CollectiblesNumber` (break `/Game/Customs/Blueprints/GameplayFrameWork/DataStructs/BPS_PlayerStateData` _value))
    (set `self.EnemiesNumber` (`.EnemiesNumber_4_450506104A2B7AAC76EAD6A271E7B61C` (break `/Game/Customs/Blueprints/GameplayFrameWork/DataStructs/BPS_PlayerStateData` _value)))
    (`self.DispatcherSetDoorOpen`)))

(event `TakeDamage`
  (bind _output_get (set `self.Energy` (- (`self.Energy`) 1.0)))
  (`self.UpdateHealthBar`)
  (if (<= _output_get 0.0)
    (`self.DispatcherDeath`)))

(event `AddEnergy`
  (set `self.Energy` (`KismetMathLibrary.FClamp` (+ (`self.Energy`) 1.0) 0.0 (`self.MaxEnergy`)))
  (`self.UpdateHealthBar`))

(fn `UpdateHealthBar`
  (`/Game/Customs/Blueprints/UI/Widget/WBP_MainHud.UpdateHealthBar` (`self.HudRef`) (`self.Energy`) (`self.MaxEnergy`)))

(fn `UpdateHudArchivement`
  (`/Game/Customs/Blueprints/UI/Widget/WBP_MainHud.UpdateArchivement` (`self.HudRef`) (`self.CollectiblesNumber`) (`self.EnemiesNumber`)))

(fn `UserConstructionScript`)