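; BP_PlayerCtrl is a player controller that turns Enhanced Input actions into commands for the controlled pawn.
; On BeginPlay it adds the IMC_Player mapping context to the local player's input subsystem.
; Move, look and jump inputs go to the pawn as interface-style messages, with no cast to a pawn class.
; End-jump fires only on the jump action's Canceled event; Completed is not handled.
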(event `self.ReceiveBeginPlay`
  (bind _returnvalue (subsystem `EnhancedInputLocalPlayerSubsystem`))
  (`/Engine/EditorBlueprintResources/StandardMacros.IsValid` _returnvalue
    (:`Is Valid`
      (`EnhancedInputSubsystemInterface.AddMappingContext` _returnvalue "/Game/Customs/Input/IMC_Player.IMC_Player" 0 (struct)))))

(event `EnhancedInput|/Game/Customs/Input/IA_MyJump`
  (params (ActionValue :type Boolean) (ElapsedSeconds :type "Float (double-precision)") (TriggeredSeconds :type "Float (double-precision)") (InputAction :type "InputAction Object Reference" :default "/Game/Customs/Input/IA_MyJump.IA_MyJump"))
  (bind _returnvalue (`self.K2_GetPawn`))
  (:`Started`
    (message `/Game/Customs/Input/Interfaces/I_InputReciver.I_Jump` _returnvalue))
  (:`Canceled`
    (message `/Game/Customs/Input/Interfaces/I_InputReciver.I_EndJump` _returnvalue)))

(event `EnhancedInput|/Game/Customs/Input/IA_MyLook`
  (params (ActionValue :type "Vector2D Structure") (ElapsedSeconds :type "Float (double-precision)") (TriggeredSeconds :type "Float (double-precision)") (InputAction :type "InputAction Object Reference" :default "/Game/Customs/Input/IA_MyLook.IA_MyLook"))
  (:`Triggered`
    (message `/Game/Customs/Input/Interfaces/I_InputReciver.I_Look` (`self.K2_GetPawn`) ActionValue_X ActionValue_Y)))

(event `EnhancedInput|/Game/Customs/Input/IA_MyMove`
  (params (ActionValue :type "Vector2D Structure") (ElapsedSeconds :type "Float (double-precision)") (TriggeredSeconds :type "Float (double-precision)") (InputAction :type "InputAction Object Reference" :default "/Game/Customs/Input/IA_MyMove.IA_MyMove"))
  (:`Triggered`
    (message `/Game/Customs/Input/Interfaces/I_InputReciver.I_Move` (`self.K2_GetPawn`) ActionValue_X ActionValue_Y)))

(fn `UserConstructionScript`)