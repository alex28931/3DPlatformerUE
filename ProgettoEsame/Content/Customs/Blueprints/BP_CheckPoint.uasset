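; Checkpoint actor that triggers a game save when the player enters its trigger box.
; On overlap it flags itself as saved, calls Save on BP_GameInstance and destroys the box, so it fires once.
; It binds to the game instance's save dispatcher to record its flag in CheckPointsData under its index.
; On BeginPlay it reads that entry back and destroys itself if already saved.
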(event `self.ReceiveBeginPlay`
  (bind _asbp_game_instance (cast `/Game/Customs/Blueprints/GameplayFrameWork/BP_GameInstance` (`GameplayStatics.GetGameInstance`)))
  (bind _output_get (set `self.GameInstanceRef` _asbp_game_instance))
  (add `/Game/Customs/Blueprints/GameplayFrameWork/BP_GameInstance.DispatcherSave` _output_get (delegate `DispatcherSave`))
  (if (`BlueprintMapLibrary.Map_Contains` (`/Game/Customs/Blueprints/GameplayFrameWork/BP_GameInstance.CheckPointsData` (`self.GameInstanceRef`)) (`self.CheckPointIndex`))
    (`self.Load`)))

(event `DispatcherSave`
  (`self.Save`))

(event `self.TriggerBox.OnComponentBeginOverlap`
  (params (OverlappedComponent :type "PrimitiveComponent Object Reference") (OtherActor :type "Actor Object Reference") (OtherComp :type "PrimitiveComponent Object Reference") (OtherBodyIndex :type Integer) (bFromSweep :type Boolean) (SweepResult :type "HitResult Structure (by ref)"))
  (if (`self.ActorHasTag` OtherActor "Player")
    (set `self.AlreadySaved` true)
    (`/Game/Customs/Blueprints/GameplayFrameWork/BP_GameInstance.Save` (`self.GameInstanceRef`))
    (`ActorComponent.K2_DestroyComponent` (`self.TriggerBox`))))

(event `Save`
  (`BlueprintMapLibrary.Map_Add` (`/Game/Customs/Blueprints/GameplayFrameWork/BP_GameInstance.CheckPointsData` (`self.GameInstanceRef`)) (`self.CheckPointIndex`) (make `/Game/Customs/Blueprints/GameplayFrameWork/DataStructs/BPS_CheckPoint` (`self.AlreadySaved`))))

(event `Load`
  (bind (_value _returnvalue) (`BlueprintMapLibrary.Map_Find` (`/Game/Customs/Blueprints/GameplayFrameWork/BP_GameInstance.CheckPointsData` (`self.GameInstanceRef`)) (`self.CheckPointIndex`)))
  (if _returnvalue
    (bind _output_get (set `self.AlreadySaved` (break `/Game/Customs/Blueprints/GameplayFrameWork/DataStructs/BPS_CheckPoint` _value)))
    (if _output_get
      (`self.K2_DestroyActor`))))

(fn `UserConstructionScript`)