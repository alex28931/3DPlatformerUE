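; AI controller for the tracker enemy that runs the BT_EnemyTracker behavior tree on possession and tracks the player through AI perception.
; Sight or touch stimuli from actors tagged Player write the actor to the PlayerRef blackboard key and cancel the pending forget timer.
; Losing either stimulus starts a five-second timer that clears PlayerRef, giving the enemy a short memory after losing contact.
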(event `self.ReceivePossess`
  (params (PossessedPawn :type "Pawn Object Reference"))
  (set `self.Possessed Pawn` PossessedPawn)
  (`self.RunBehaviorTree` "/Game/Customs/Blueprints/Enemies/AI/AIEnemyTracker/BT_EnemyTracker.BT_EnemyTracker"))

(event `self.AIPerception.OnTargetPerceptionUpdated`
  (params (Actor :type "Actor Object Reference") (Stimulus :type "AIStimulus Structure"))
  (if (`self.ActorHasTag` Actor "Player")
    (set `self.PerceivedActor` Actor)
    (bind _returnvalue (`AIPerceptionSystem.GetSenseClassForStimulus` Stimulus))
    (if (or (== _returnvalue "/Script/AIModule.AISense_Sight") (== _returnvalue "/Script/AIModule.AISense_Touch"))
      (if (`.bSuccessfullySensed` (break `AIStimulus` Stimulus))
        (`KismetSystemLibrary.K2_ClearAndInvalidateTimerHandle` (`self.LineOfSightTimer`))
        (`BlackboardComponent.SetValueAsObject` (`self.Blackboard`) "PlayerRef" (`self.PerceivedActor`))
        (else
          (bind _returnvalue_2 (`KismetSystemLibrary.K2_SetTimerDelegate` (delegate `EndTimer`) 5.0))
          (set `self.LineOfSightTimer` _returnvalue_2))))))

(event `EndTimer`
  (`BlackboardComponent.SetValueAsObject` (`self.Blackboard`) "PlayerRef" null))

(fn `UserConstructionScript`)