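; AI controller for the shooter enemy that runs its behavior tree on possession and reacts to perceiving the player.
; Sight or touch detection stores the player in the blackboard and starts a looping timer that allows ranged attacks within a mid-distance band.
; Losing the player stops that check, disables ranged attack and starts a delay that clears the player reference unless the player is sensed again.
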(event `self.ReceivePossess`
  (params (PossessedPawn :type "Pawn Object Reference"))
  (set `self.Possessed Pawn` PossessedPawn)
  (`self.RunBehaviorTree` "/Game/Customs/Blueprints/Enemies/AI/AI_EnemyShooter/BT_EnemyShooter.BT_EnemyShooter"))

(event `self.AIPerception.OnTargetPerceptionUpdated`
  (params (Actor :type "Actor Object Reference") (Stimulus :type "AIStimulus Structure"))
  (if (`self.ActorHasTag` Actor "Player")
    (set `self.PerceivedActor` Actor)
    (bind _returnvalue (`AIPerceptionSystem.GetSenseClassForStimulus` Stimulus))
    (if (or (== _returnvalue "/Script/AIModule.AISense_Sight") (== _returnvalue "/Script/AIModule.AISense_Touch"))
      (if (`.bSuccessfullySensed` (break `AIStimulus` Stimulus))
        (`KismetSystemLibrary.K2_ClearAndInvalidateTimerHandle` (`self.LineOfSightTimer`))
        (`BlackboardComponent.SetValueAsObject` (`self.Blackboard`) (`self.PlayerRef`) (`self.PerceivedActor`))
        (bind _returnvalue_2 (`KismetSystemLibrary.K2_SetTimerDelegate` (delegate `CheckDistanceForAttack`) 0.5 true))
        (set `self.TimerForCheckDistanceForAttack` _returnvalue_2)
        (else
          (bind _returnvalue_3 (`KismetSystemLibrary.K2_SetTimerDelegate` (delegate `EndTimer`) 10.0))
          (set `self.LineOfSightTimer` _returnvalue_3)
          (`KismetSystemLibrary.K2_ClearAndInvalidateTimerHandle` (`self.TimerForCheckDistanceForAttack`))
          (`BlackboardComponent.SetValueAsBool` (`self.Blackboard`) (`self.CanUseRangedAttack`) false))))))

(event `CheckDistanceForAttack`
  (bind _returnvalue (`KismetMathLibrary.Vector_Distance` (`self.K2_GetActorLocation` (`self.Possessed Pawn`)) (`self.K2_GetActorLocation` (`self.PerceivedActor`))))
  (`BlackboardComponent.SetValueAsBool` (`self.Blackboard`) (`self.CanUseRangedAttack`) (and (<= _returnvalue 1500.0) (>= _returnvalue 500.0))))

(event `EndTimer`
  (`BlackboardComponent.SetValueAsObject` (`self.Blackboard`) "PlayerRef" null))

(fn `UserConstructionScript`)