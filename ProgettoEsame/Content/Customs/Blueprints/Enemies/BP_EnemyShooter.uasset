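; BP_EnemyShooter is a ranged enemy that fires BP_Projectile from its left hand.
; On BeginPlay it runs parent logic, then snaps LeftHandCollider to the left hand socket on the mesh.
; Interface-style events start and stop the left attack section of the mutant attack montage.
; A separate ISpawnProjectile event spawns the projectile at the collider's world transform, keeping animation and firing decoupled.
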(event `self.ReceiveBeginPlay`
  (`parent.ReceiveBeginPlay`)
  (`SceneComponent.K2_AttachToComponent` (`self.LeftHandCollider`) (`self.Mesh`) "LeftHandSocket" "SnapToTarget" "SnapToTarget" "KeepRelative" true))

(event `/Game/Customs/Blueprints/Enemies/AI/Interfaces/I_AI.I_RangedAttack`
  (`self.PlayAnimMontage` "/Game/Customs/Enemies/Mutant/Animations/AM_MutantAttack.AM_MutantAttack" 1.0 "LeftAttack"))

(event `/Game/Customs/Blueprints/Enemies/AI/Interfaces/I_AI.I_StopRangedAttack`
  (`self.StopAnimMontage` "/Game/Customs/Enemies/Mutant/Animations/AM_MutantAttack.AM_MutantAttack"))

(event `/Game/Customs/Blueprints/Interfaces/I_AnimNotify.I_SpawnProjectile`
  (`|SpawnActorFromClass` "/Game/Customs/Blueprints/Object/BP_Projectile.BP_Projectile_C" (`SceneComponent.K2_GetComponentToWorld` (`self.LeftHandCollider`)) "Undefined" "MultiplyWithRoot" null null))

(fn `UserConstructionScript`
  (`parent.UserConstructionScript`))