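; Walking enemy that exposes its path component's targets and a walk-speed setter through interfaces.
; On capsule hit it reports an AI touch event and sends the other actor a launch impulse with its head position, dying if that call returns true.
; Death disables and hides it, notifies the killer and randomly drops an energy or invulnerability pickup.
; Defeat state saves to the GameInstance by EnemyIndex, destroying defeated walkers on load.
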(event `self.ReceiveBeginPlay`
  (bind _asbp_game_instance (cast `/Game/Customs/Blueprints/GameplayFrameWork/BP_GameInstance` (`GameplayStatics.GetGameInstance`)))
  (bind _output_get (set `self.GameInstanceRef` _asbp_game_instance))
  (add `/Game/Customs/Blueprints/GameplayFrameWork/BP_GameInstance.DispatcherSave` _output_get (delegate `DispatcherSave`))
  (if (`BlueprintMapLibrary.Map_Contains` (`/Game/Customs/Blueprints/GameplayFrameWork/BP_GameInstance.EnemiesData` (`self.GameInstanceRef`)) (`self.EnemyIndex`))
    (`self.Load`)))

(event `DispatcherSave`
  (`self.Save`))

(event `self.CapsuleComponent.OnComponentHit`
  (params (HitComponent :type "PrimitiveComponent Object Reference") (OtherActor :type "Actor Object Reference") (OtherComp :type "PrimitiveComponent Object Reference") (NormalImpulse :type "Vector Structure") (Hit :type "HitResult Structure (by ref)"))
  (`AISense_Touch.ReportTouchEvent` self OtherActor Hit_Location)
  (bind _charisup (message `/Game/Customs/Blueprints/Interfaces/I_Damage.I_EnemyLaunchCharacter` OtherActor (* (`KismetMathLibrary.Normal` (- (`self.K2_GetActorLocation` OtherActor) (`self.K2_GetActorLocation`))) 1200.0) (`SceneComponent.K2_GetComponentLocation` (`self.HeadPos`))))
  (if _charisup
    (`self.Death` OtherActor)))

(event `Death`
  (params (Actor :type "Actor Object Reference"))
  (bind _returnvalue (`self.GetTransform`))
  (bind _mesh (`self.Mesh`))
  (`KismetSystemLibrary.Delay` 0.1)
  (set `self.AlreadyDefeated` true)
  (`PrimitiveComponent.SetCollisionEnabled` (`self.CapsuleComponent`) "NoCollision")
  (`CharacterMovementComponent.DisableMovement` (`self.CharacterMovement`))
  (`SkeletalMeshComponent.SetAnimInstanceClass` _mesh null)
  (`SceneComponent.SetVisibility` _mesh false false)
  (`PrimitiveComponent.SetCollisionEnabled` _mesh "NoCollision")
  (message `/Game/Customs/Blueprints/Interfaces/I_AddArchivement.I_AddEnemy` Actor)
  (if (== (`KismetMathLibrary.RandomIntegerInRange` 1 3) 1)
    (if (`KismetMathLibrary.RandomBool`)
      (`|SpawnActorFromClass` "/Game/Customs/Blueprints/Object/BP_PUEnergy.BP_PUEnergy_C" _returnvalue "Undefined" "MultiplyWithRoot" null null)
      (else
        (`|SpawnActorFromClass` "/Game/Customs/Blueprints/Object/BP_PUInvulnerability.BP_PUInvulnerability_C" _returnvalue "Undefined" "MultiplyWithRoot" null null)))))

(event `Save`
  (`BlueprintMapLibrary.Map_Add` (`/Game/Customs/Blueprints/GameplayFrameWork/BP_GameInstance.EnemiesData` (`self.GameInstanceRef`)) (`self.EnemyIndex`) (make `/Game/Customs/Blueprints/GameplayFrameWork/DataStructs/BPS_EnemyData` (`self.AlreadyDefeated`))))

(event `Load`
  (bind (_value _returnvalue) (`BlueprintMapLibrary.Map_Find` (`/Game/Customs/Blueprints/GameplayFrameWork/BP_GameInstance.EnemiesData` (`self.GameInstanceRef`)) (`self.EnemyIndex`)))
  (if _returnvalue
    (if (break `/Game/Customs/Blueprints/GameplayFrameWork/DataStructs/BPS_EnemyData` _value)
      (`self.K2_DestroyActor`))))

(event `/Game/Customs/Blueprints/Enemies/AI/Interfaces/I_AI.I_ChangeMaxWalkSpeed`
  (params (MaxWalkSpeed :type "Float (double-precision)"))
  (set `CharacterMovementComponent.MaxWalkSpeed` MaxWalkSpeed (`self.CharacterMovement`)))

(fn `I_GetTargetList`
  (returns (NewParam :type "Array of /Game/Customs/Blueprints/Enemies/AI/BP_PathTarget Object Reference"))
  (return (`/Game/Customs/Blueprints/Enemies/AI/BP_PathComponent.TargetList` (`self.BP_PathComponent`))))

(fn `UserConstructionScript`)