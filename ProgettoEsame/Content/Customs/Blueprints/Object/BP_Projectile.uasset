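; BP_Projectile is a projectile that flies toward the player and knocks them back on impact.
; It locks its direction toward player character 0 at BeginPlay, then moves straight at Speed each Tick with a swept SetActorLocation, without homing.
; On mesh hit, it sends an upward-biased launch vector to valid actors tagged Player through an interface message, then destroys itself on any hit.
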(event `self.ReceiveBeginPlay`
  (set `self.Direction` (`KismetMathLibrary.Normal` (- (`self.K2_GetActorLocation` (`GameplayStatics.GetPlayerCharacter` 0)) (`self.K2_GetActorLocation`)))))

(event `self.ReceiveTick`
  (params (DeltaSeconds :type "Float (single-precision)"))
  (`self.K2_SetActorLocation` (+ (`self.K2_GetActorLocation`) (* (`self.Direction`) (* DeltaSeconds (`self.Speed`)))) true))

(event `self.StaticMesh.OnComponentHit`
  (params (HitComponent :type "PrimitiveComponent Object Reference") (OtherActor :type "Actor Object Reference") (OtherComp :type "PrimitiveComponent Object Reference") (NormalImpulse :type "Vector Structure") (Hit :type "HitResult Structure (by ref)"))
  (`/Engine/EditorBlueprintResources/StandardMacros.IsValid` OtherActor
    (:`Is Valid`
      (if (`self.ActorHasTag` OtherActor "Player")
        (message `/Game/Customs/Blueprints/Interfaces/I_Damage.I_ProjectileLauchCharacter` OtherActor (* (`KismetMathLibrary.Normal` (+ (`KismetMathLibrary.Normal` (- (`self.K2_GetActorLocation` OtherActor) (`self.K2_GetActorLocation`))) (0.0 0.0 0.3))) 1200.0))))
    (:`Is Not Valid`
      _))
  (`self.K2_DestroyActor`))

(fn `UserConstructionScript`)