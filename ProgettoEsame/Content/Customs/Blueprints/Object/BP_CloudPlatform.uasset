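; BP_CloudPlatform is a cloud platform that toggles its collision to act as a pass-through platform from below.
; The ICheckLocation event disables collision on the Platform and Cloud components when the supplied location is at or below the Platform's height.
; An actor tagged Player leaving the box trigger restores query and physics collision on both components.
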(event `/Game/Customs/Blueprints/Interfaces/I_CheckCollision.I_CheckLocation`
  (params (Location :type "Vector Structure"))
  (bind (_returnvalue_x _returnvalue_y _returnvalue_z) (`KismetMathLibrary.BreakVector` (`SceneComponent.K2_GetComponentLocation` (`self.Platform`))))
  (if (<= Location_Z _returnvalue_z)
    (`PrimitiveComponent.SetCollisionEnabled` (`self.Platform`) "NoCollision")
    (`PrimitiveComponent.SetCollisionEnabled` (`self.Cloud`) "NoCollision")))

(event `self.Box_0.OnComponentEndOverlap`
  (params (OverlappedComponent :type "PrimitiveComponent Object Reference") (OtherActor :type "Actor Object Reference") (OtherComp :type "PrimitiveComponent Object Reference") (OtherBodyIndex :type Integer))
  (if (`self.ActorHasTag` OtherActor "Player")
    (`PrimitiveComponent.SetCollisionEnabled` (`self.Platform`) "QueryAndPhysics")
    (`PrimitiveComponent.SetCollisionEnabled` (`self.Cloud`) "QueryAndPhysics")))

(fn `UserConstructionScript`
  (`parent.UserConstructionScript`))