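; BP_Gate is a double-leaf gate that opens once the player state's enemy and collectible counts reach its thresholds.
; On BeginPlay it caches BP_PlayerState and binds Open and SetDoorOpen to its dispatchers.
; Open swings both pivots in mirrored directions through a timeline rotation lerp.
; SetDoorOpen applies the same threshold check, snaps the pivots to the end rotation and sets AlreadyOpen, which blocks later animated opening.
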(event `SetDoorOpen`
  (bind _endrot (`self.EndRot`))
  (if (and (>= (`/Game/Customs/Blueprints/GameplayFrameWork/BP_PlayerState.EnemiesNumber` (`self.PlayerStateRef`)) (`self.EnemiesToOpen`)) (>= (`/Game/Customs/Blueprints/GameplayFrameWork/BP_PlayerState.CollectiblesNumber` (`self.PlayerStateRef`)) (`self.CollectiblesToOpen`)))
    (`SceneComponent.K2_SetRelativeRotation` (`self.PivotL`) _endrot false false)
    (`SceneComponent.K2_SetRelativeRotation` (`self.PivotR`) (* _endrot -1.0) false false)
    (set `self.AlreadyOpen` true)))

(event `self.ReceiveBeginPlay`
  (bind _asbp_player_state (cast `/Game/Customs/Blueprints/GameplayFrameWork/BP_PlayerState` (`GameplayStatics.GetPlayerState` 0)))
  (bind _output_get (set `self.PlayerStateRef` _asbp_player_state))
  (add `/Game/Customs/Blueprints/GameplayFrameWork/BP_PlayerState.DispatcherOpen` _output_get (delegate `Open`))
  (add `/Game/Customs/Blueprints/GameplayFrameWork/BP_PlayerState.DispatcherSetDoorOpen` (`self.PlayerStateRef`) (delegate `SetDoorOpen`)))

(event `Open`
  (if (and (>= (`/Game/Customs/Blueprints/GameplayFrameWork/BP_PlayerState.EnemiesNumber` (`self.PlayerStateRef`)) (`self.EnemiesToOpen`)) (>= (`/Game/Customs/Blueprints/GameplayFrameWork/BP_PlayerState.CollectiblesNumber` (`self.PlayerStateRef`)) (`self.CollectiblesToOpen`)) (not (`self.AlreadyOpen`)))
    (bind (_direction _alpha) (`Timeline|Timeline_0`)
      (:`Update`
        (bind _returnvalue (`KismetMathLibrary.RLerp` (`self.StartRot`) (`self.EndRot`) _alpha))
        (`SceneComponent.K2_SetRelativeRotation` (`self.PivotL`) _returnvalue false false)
        (`SceneComponent.K2_SetRelativeRotation` (`self.PivotR`) (* _returnvalue -1.0) false false)))))

(fn `UserConstructionScript`)