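; BP_Block is a breakable block actor that can drop a random power-up when something overlaps it.
; A TriggerBox overlap waits briefly, then disables collision on the trigger and the block and hides the block rather than destroying it.
; SpawnRandomPU then has a one-in-three chance to spawn either an energy or an invulnerability power-up, picked at random, at the block's transform.
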(event `self.TriggerBox.OnComponentBeginOverlap`
  (params (OverlappedComponent :type "PrimitiveComponent Object Reference") (OtherActor :type "Actor Object Reference") (OtherComp :type "PrimitiveComponent Object Reference") (OtherBodyIndex :type Integer) (bFromSweep :type Boolean) (SweepResult :type "HitResult Structure (by ref)"))
  (bind _returnvalue (`self.GetTransform`))
  (bind _block (`self.Block`))
  (`KismetSystemLibrary.Delay` 0.3)
  (`PrimitiveComponent.SetCollisionEnabled` (`self.TriggerBox`) "NoCollision")
  (`PrimitiveComponent.SetCollisionEnabled` _block "NoCollision")
  (`SceneComponent.SetVisibility` _block false false)
  (if (== (`KismetMathLibrary.RandomIntegerInRange` 1 3) 1)
    (if (`KismetMathLibrary.RandomBool`)
      (`|SpawnActorFromClass` "/Game/Customs/Blueprints/Object/BP_PUEnergy.BP_PUEnergy_C" _returnvalue "Undefined" "MultiplyWithRoot" null null)
      (else
        (`|SpawnActorFromClass` "/Game/Customs/Blueprints/Object/BP_PUInvulnerability.BP_PUInvulnerability_C" _returnvalue "Undefined" "MultiplyWithRoot" null null)))))

(fn `UserConstructionScript`)