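; BP_Platform is a moving platform that shuttles between its spawn location and an EndPos component, pausing at each stop.
; A Timeline, rate-scaled by Velocity, lerps location with sweep and relative rotation between StartRotation and EndRotation.
; It starts on BeginPlay, or after a delay when a Player-tagged actor overlaps its trigger if HasTriggerToactivate is set.
; On Timeline completion, a FlipFlop alternates reverse and forward playback after TimeForStay.
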(event `self.ReceiveBeginPlay`
  (set `self.StartPosition` (`self.K2_GetActorLocation`))
  (set `self.EndPosition` (`SceneComponent.K2_GetComponentLocation` (`self.EndPos`)))
  (`TimelineComponent.SetPlayRate` (`self.Timeline`) (`self.Velocity`))
  (if (not (`self.HasTriggerToactivate`))
    (`self.Play`)
    (`ActorComponent.K2_DestroyComponent` (`self.TriggerToActivate`))))

(event `self.TriggerToActivate.OnComponentBeginOverlap`
  (params (OverlappedComponent :type "PrimitiveComponent Object Reference") (OtherActor :type "Actor Object Reference") (OtherComp :type "PrimitiveComponent Object Reference") (OtherBodyIndex :type Integer) (bFromSweep :type Boolean) (SweepResult :type "HitResult Structure (by ref)"))
  (if (`self.ActorHasTag` OtherActor "Player")
    (`KismetSystemLibrary.Delay` (`self.DelayForactivate`))
    (`self.Play`)))

(event `Play`
  (bind (_direction _alpha) (`Timeline|Timeline` :!label _label)
    (:`Update`
      (`self.K2_SetActorLocation` (`KismetMathLibrary.VLerp` (`self.StartPosition`) (`self.EndPosition`) _alpha) true)
      (`self.K2_SetActorRelativeRotation` (`KismetMathLibrary.RLerp` (`self.StartRotation`) (`self.EndRotation`) _alpha)))
    (:`Finished`
      (`KismetSystemLibrary.Delay` (`self.TimeForStay`))
      (`/Engine/EditorBlueprintResources/StandardMacros.FlipFlop`
        (:`A`
          (`self.Reverse`))
        (:`B`
          (`self.Play`))))))

(event `Reverse`
  (goto _label :!via `Reverse`))

(fn `UserConstructionScript`)